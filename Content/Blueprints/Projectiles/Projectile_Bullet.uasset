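; Bullet projectile Blueprint that damages actors it overlaps and limits how often it can bounce.
; On overlap, the authority applies Damage to the other actor and destroys the bullet.
; Projectile movement bounce events drive a server-side Bounces counter, so with a zero starting count the first bounce is allowed and the second destroys the bullet.
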(event `self.ReceiveBeginPlay`
  (`parent.ReceiveBeginPlay`))

(event `self.ReceiveActorBeginOverlap`
  (params (OtherActor :type "Actor Object Reference"))
  (`parent.ReceiveActorBeginOverlap` OtherActor)
  (`/Engine/EditorBlueprintResources/ActorMacros.Switch Has Authority`
    (:`Authority`
      (`GameplayStatics.ApplyDamage` OtherActor (`self.Damage`))
      (`self.K2_DestroyActor`))))

(event `self.ProjectileMovement.OnProjectileBounce`
  (params (ImpactResult :type "HitResult Structure (by ref)") (ImpactVelocity :type "Vector Structure (by ref)"))
  (bind _bounces (`self.Bounces`))
  ;[1 1 1] Destroy after more than 1 bounce
  (`/Engine/EditorBlueprintResources/ActorMacros.Switch Has Authority`
    (:`Authority`
      (if (>= _bounces 1)
        (`self.K2_DestroyActor`)
        (else
          (set `self.Bounces` (+ _bounces 2)))))))

(fn `UserConstructionScript`
  (`parent.UserConstructionScript`))