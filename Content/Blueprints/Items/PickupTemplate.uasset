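; Template pickup item that shows a HUD prompt when the player is nearby and can add health.
; Trigger overlap with a ThirdPersonCharacter toggles IsInRange and pushes the ItemInfo text and visibility to that character's HUD reference.
; UseAction adds AddHealth to player 0's Health, without checking IsInRange, clamping the value or removing the pickup.
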(event `UpdatePickupText`
  (params (IsVisible :type "ESlateVisibility Enum" :default "Visible") (Player :type "/Game/ThirdPersonBP/Blueprints/ThirdPersonCharacter Object Reference"))
  (bind _gamehudreference (`/Game/ThirdPersonBP/Blueprints/ThirdPersonCharacter.GameHudReference` Player))
  ;[1 1 1] Update Pickup Text
  (set `/Game/UMG/GameHUD.PickupTextValue` (`.PickupText_12_EC983FB947AD4DACE538F686D8A39BDE` (break `/Game/ThirdPersonBP/Blueprints/InventoryStruct` (`self.ItemInfo`))) _gamehudreference)
  (set `/Game/UMG/GameHUD.PickupTextVisible` IsVisible _gamehudreference))

(event `self.Trigger.OnComponentBeginOverlap`
  (params (OverlappedComponent :type "PrimitiveComponent Object Reference") (OtherActor :type "Actor Object Reference") (OtherComp :type "PrimitiveComponent Object Reference") (OtherBodyIndex :type Integer) (bFromSweep :type Boolean) (SweepResult :type "HitResult Structure (by ref)"))
  ;[1 1 1] Overlap Trigger Script
  (bind _asthird_person_character (cast `/Game/ThirdPersonBP/Blueprints/ThirdPersonCharacter` OtherActor))
  (`self.UpdatePickupText` "Visible" _asthird_person_character)
  (set `self.IsInRange?` true))

(event `self.Trigger.OnComponentEndOverlap`
  (params (OverlappedComponent :type "PrimitiveComponent Object Reference") (OtherActor :type "Actor Object Reference") (OtherComp :type "PrimitiveComponent Object Reference") (OtherBodyIndex :type Integer))
  ;[1 1 1] Overlap Trigger Script
  (bind _asthird_person_character (cast `/Game/ThirdPersonBP/Blueprints/ThirdPersonCharacter` OtherActor))
  (`self.UpdatePickupText` "Hidden" _asthird_person_character)
  (set `self.IsInRange?` false))

(event `/Game/ThirdPersonBP/Blueprints/ActionInterface.UseAction`
  ;[1 1 1] Use Action
  (bind _asthird_person_character (cast `/Game/ThirdPersonBP/Blueprints/ThirdPersonCharacter` (`GameplayStatics.GetPlayerCharacter` 0)))
  (set `/Game/ThirdPersonBP/Blueprints/ThirdPersonCharacter.Health` (+ (`/Game/ThirdPersonBP/Blueprints/ThirdPersonCharacter.Health` _asthird_person_character) (`self.AddHealth`)) _asthird_person_character))

(fn `UserConstructionScript`)