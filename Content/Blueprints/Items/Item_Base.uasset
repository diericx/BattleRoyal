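; Base item actor that players can focus on, pick up into their inventory and use to add health.
; Trigger overlaps split by authority: the server sets or clears the character's FocusedItem, while remote clients toggle the item's HUD name for the local character.
; PickupItem stores ItemInfo and hides the actor, but its condition includes a constant false, so it never executes.
; AttemptToUseItem adds AddHealth and destroys the item; its in-file call is disconnected.
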(event `self.ReceiveBeginPlay`
  ;[1 1 1] Event begin play
  (setmembers `/Game/Blueprints/UI/InventoryStruct` :`StructRef` (`self.ItemInfo`) :`Item` self)
  (bind _asthird_person_character (cast `/Game/ThirdPersonBP/Blueprints/ThirdPersonCharacter` (`GameplayStatics.GetPlayerCharacter` 0)))
  (set `self.CharacterRef` _asthird_person_character))

(event `PickupItem`
  (params (CharRef :type "Actor Object Reference") (ItemRef :type "Actor Object Reference"))
  ;[1 0.1335 0.1036] Pickup Item
  (bind _asitem_base (cast `/Game/Blueprints/Items/Item_Base` ItemRef))
  (bind _asthird_person_character (cast `/Game/ThirdPersonBP/Blueprints/ThirdPersonCharacter` CharRef))
  (if (and (`self.GetActorEnableCollision` _asitem_base) false)
    (`KismetArrayLibrary.Array_Add` (`/Game/ThirdPersonBP/Blueprints/ThirdPersonCharacter.Inventory` _asthird_person_character) (`/Game/Blueprints/Items/Item_Base.ItemInfo` _asitem_base))
    (`self.SetActorHiddenInGame` _asitem_base true)
    (`self.SetActorEnableCollision` _asitem_base false)))

(event `self.Trigger.OnComponentBeginOverlap`
  (params (OverlappedComponent :type "PrimitiveComponent Object Reference") (OtherActor :type "Actor Object Reference") (OtherComp :type "PrimitiveComponent Object Reference") (OtherBodyIndex :type Integer) (bFromSweep :type Boolean) (SweepResult :type "HitResult Structure (by ref)"))
  ;[1 1 1] Overlap Trigger
  (if (not (`self.bHidden`))
    (`/Engine/EditorBlueprintResources/ActorMacros.Switch Has Authority`
      (:`Authority`
        ;;[1 0.1335 0.1036] Set focused item
        (bind _asthird_person_character (cast `/Game/ThirdPersonBP/Blueprints/ThirdPersonCharacter` OtherActor))
        (set `/Game/ThirdPersonBP/Blueprints/ThirdPersonCharacter.FocusedItem` self _asthird_person_character)
        (`KismetSystemLibrary.PrintString` "set focused item"))
      (:`Remote`
        (bind _asthird_person_character_2 (cast `/Game/ThirdPersonBP/Blueprints/ThirdPersonCharacter` OtherActor))
        (if (== _asthird_person_character_2 (`self.CharacterRef`))
          (bind _hudref (`/Game/ThirdPersonBP/Blueprints/ThirdPersonCharacter.HUDRef` _asthird_person_character_2))
          (set `/Game/Blueprints/UI/HUD.FocusedItemText` (`.Name_12_ACA8D398490F27A527935DBEAE3FAB24` (break `/Game/Blueprints/UI/InventoryStruct` (`self.ItemInfo`))) _hudref)
          (set `/Game/Blueprints/UI/HUD.FocusedItemTextVisibility` "Visible" _hudref))))))

(event `self.Trigger.OnComponentEndOverlap`
  (params (OverlappedComponent :type "PrimitiveComponent Object Reference") (OtherActor :type "Actor Object Reference") (OtherComp :type "PrimitiveComponent Object Reference") (OtherBodyIndex :type Integer))
  ;[1 1 1] Overlap Trigger
  (`/Engine/EditorBlueprintResources/ActorMacros.Switch Has Authority`
    (:`Authority`
      ;;[1 0.1335 0.1036] remove focused item
      (bind _asthird_person_character (cast `/Game/ThirdPersonBP/Blueprints/ThirdPersonCharacter` OtherActor))
      (set `/Game/ThirdPersonBP/Blueprints/ThirdPersonCharacter.FocusedItem` null _asthird_person_character)
      (`KismetSystemLibrary.PrintString` "removed focused item"))
    (:`Remote`
      (bind _asthird_person_character_2 (cast `/Game/ThirdPersonBP/Blueprints/ThirdPersonCharacter` OtherActor))
      (if (== _asthird_person_character_2 (`self.CharacterRef`))
        (set `/Game/Blueprints/UI/HUD.FocusedItemTextVisibility` "Hidden" (`/Game/ThirdPersonBP/Blueprints/ThirdPersonCharacter.HUDRef` _asthird_person_character_2))))))

(event `AttemptToUseItem`
  (params (CharRef :type "Actor Object Reference") (ItemRef :type "Actor Object Reference"))
  ;[1 0.1335 0.1036] Use a player's item
  (bind _asitem_base (cast `/Game/Blueprints/Items/Item_Base` ItemRef))
  (bind _asthird_person_character (cast `/Game/ThirdPersonBP/Blueprints/ThirdPersonCharacter` CharRef))
  (set `/Game/ThirdPersonBP/Blueprints/ThirdPersonCharacter.Health` (+ (`/Game/ThirdPersonBP/Blueprints/ThirdPersonCharacter.Health` _asthird_person_character) (`/Game/Blueprints/Items/Item_Base.AddHealth` _asitem_base)) _asthird_person_character)
  (`self.K2_DestroyActor` ItemRef))

(fn `UserConstructionScript`)